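; A crusher trap for a 2D side-scroller that punches down from its placed position and rises back, damaging the player character.
; Tick moves it with a swept SetActorLocation at separate down and up speeds, flipping direction and pausing at each end of its travel.
; Hit and overlap events share one branch that applies 1000 damage to the character only while the direction is downward.
; The construction script moves an arrow component to mark the travel distance.
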(event EventBeginPlay
  (bind _returnvalue (Transformation|GetActorLocation))
  (bind _z (Math|Vector|BreakVector _returnvalue))
  (Variables|Default|Setzmin _z)
  (Variables|Default|Setzmax (- _z (Variables|Default|Gettravel_dist))))

(event EventTick
  (params (DeltaSeconds :type Float%20%28single-precision%29))
  (bind _returnvalue (Transformation|GetActorLocation))
  (bind (_x _y _z) (Math|Vector|BreakVector _returnvalue))
  (Variables|Default|Setdt DeltaSeconds)
  (Utilities|FlowControl|Sequence
    (:then_0
      (if (<= (Variables|Default|Getwait) 0.0)
        (if (< (Variables|Default|Getk) 0.0)
          (Variables|Default|Setcspd (Variables|Default|Getspd_down))
          (else
            (Variables|Default|Setcspd (Variables|Default|Getspd_up))))))
    (:then_1
      (if (<= (Variables|Default|Getwait) 0.0)
        (if (and (< (Variables|Default|Getk) 0.0) (> (.Z (Math|Vector|BreakVector (Transformation|GetActorLocation))) (Variables|Default|Getzmax)))
          (Transformation|SetActorLocation (Math|Vector|MakeVector _x _y (+ _z (* (Variables|Default|Getk) (Variables|Default|Getcspd) (Variables|Default|Getdt)))) true false :!label _label)
          (elif (and (> (Variables|Default|Getk) 0.0) (< (.Z (Math|Vector|BreakVector (Transformation|GetActorLocation))) (Variables|Default|Getzmin)))
            (goto _label)
            (else
              (Variables|Default|Setk (* (Variables|Default|Getk) -1.0))
              (Variables|Default|Setwait (Variables|Default|Getwaittime)))))
        (else
          (Variables|Default|Setwait (- (Variables|Default|Getwait) (Variables|Default|Getdt))))))))

(event Collision|EventActorBeginOverlap
  (params (OtherActor :type Actor%20Object%20Reference))
  (Utilities|Casting|CastToBP_2DSideScrollerCharacter OtherActor)
  (if (== (Variables|Default|Getk) -1.0)
    (Class|GBJamCharacter|ApplyDamage (stale Collision|EventHit _asbp_2dside_scroller_character) 1000)))

(event Collision|EventHit
  (params (MyComp :type Primitive%20Component%20Object%20Reference) (Other :type Actor%20Object%20Reference) (OtherComp :type Primitive%20Component%20Object%20Reference) (bSelfMoved :type Boolean) (HitLocation :type Vector :default "0, 0, 0") (HitNormal :type Vector :default "0, 0, 0") (NormalImpulse :type Vector :default "0, 0, 0") (Hit :type Hit%20Result%20Structure%20%28by%20ref%29))
  (bind _asbp_2dside_scroller_character (Utilities|Casting|CastToBP_2DSideScrollerCharacter Other))
  (if (== (Variables|Default|Getk) -1.0)
    (Class|GBJamCharacter|ApplyDamage _asbp_2dside_scroller_character 1000)))

(fn ConstructionScript
  (Transformation|SetRelativeLocation (Variables|Default|GetArrow) (Math|Vector|MakeVector 0.0 0.0 (* (Variables|Default|Gettravel_dist) -1.0)) false false))
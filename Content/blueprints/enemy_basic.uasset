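; Basic Paper2D enemy that approaches the player and fires projectiles in range, but its main logic is unwired: Tick and ColorRestore are empty.
; BeginPlay times attacks from flipbook lengths; AnyDamage subtracts health and tints the sprite.
; The disconnected graph holds a timer-gated idle/walk/telegraph/attack state machine, end-of-loop animation switching and death cleanup.
; Walk steps use a downward ledge trace, bypassed by Suicidal; unwired tint recovery would grant invulnerability.
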(event EventBeginPlay
  (bind _paperflipbook (Variables|Default|GetPaperFlipbook))
  (bind _paperflipbook_2 (Variables|Default|GetPaperFlipbook))
  (bind _output_get (Variables|Default|Setcloc (Transformation|GetActorLocation)))
  (bind _output_get_2 (Variables|Default|Settarg _output_get))
  (Variables|Default|Setstart _output_get_2)
  (Variables|Default|Setstatus 0)
  (Sprite|SetFlipbook _paperflipbook_2 (Variables|Default|Gettelegraph_anim))
  (Variables|Default|Settelegraph_length (Class|PaperFlipbookComponent|GetFlipbookLength _paperflipbook_2))
  (Sprite|SetFlipbook _paperflipbook (Variables|Default|Getattack_anim))
  (Variables|Default|Setatt_reload (Class|PaperFlipbookComponent|GetFlipbookLength _paperflipbook))
  (Sprite|SetFlipbook (Variables|Default|GetPaperFlipbook) (Variables|Default|Getstand_anim)))

(event Collision|EventActorBeginOverlap
  (params (OtherActor :type Actor%20Object%20Reference)))

(event EventTick
  (params (DeltaSeconds :type Float%20%28single-precision%29)))

(event Game|Damage|EventAnyDamage
  (params (Damage :type Float%20%28single-precision%29) (DamageType :type Damage%20Type%20Object%20Reference) (InstigatedBy :type Controller%20Object%20Reference) (DamageCauser :type Actor%20Object%20Reference))
  (if (and (not (Variables|Default|Getinvuln)) (> (Variables|Default|Gethp) 0.0))
    (Variables|Default|Sethp (- (Variables|Default|Gethp) Damage))
    (Sprite|SetSpriteColor (Variables|Default|GetPaperFlipbook) (Utilities|Struct|MakeLinearColor 1.0 0.0 0.0 1.0))))

(fn ConstructionScript)

(fn ColorRestore)

(fn Getdisttoplayer
  (return (Math|Vector|VectorLength (- (Transformation|GetActorLocation (Game|Player|GetPlayerPawn 0)) (Transformation|GetActorLocation)))))

(fn Getdirtoplayer
  (if (>= (.X (Math|Vector|BreakVector (- (Transformation|GetActorLocation) (Transformation|GetActorLocation (Game|Player|GetPlayerPawn 0))))) 0.0)
    (return 1.0)
    (else
      (return -1.0))))

(fn Trytowalk
  (params (kx :type Float%20%28single-precision%29) (td :type Float%20%28single-precision%29))
  (bind _returnvalue (Transformation|GetActorLocation))
  (bind (_x _y _z) (Math|Vector|BreakVector _returnvalue))
  (LocalVariables|Setkxl kx)
  (LocalVariables|Settdl td)
  (bind _returnvalue_2 (Collision|LineTraceByChannel (Math|Vector|MakeVector (+ (* (LocalVariables|Getkxl) (LocalVariables|Gettdl) -1.0) _x) _y _z) (Math|Vector|MakeVector (+ (* (LocalVariables|Getkxl) (LocalVariables|Gettdl) -1.0) _x) _y (- _z 25.0)) "TraceTypeQuery1" false 0 "None"))
  (if (or _returnvalue_2 (Variables|Default|Getsuicidal))
    (Variables|Default|Settarg (Math|Vector|MakeVector (+ (* (LocalVariables|Getkxl) (LocalVariables|Gettdl) -1.0) _x) _y _z))
    (Variables|Default|Setstart (Variables|Default|Getcloc))))